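; Master enemy Blueprint for AI-driven melee enemies with level-scaled HP, XP rewards and random power-up drops.
; BeginPlay catches HP up to the enemy level through the spawner's per-class map and pre-rolls the drop.
; Events feed the Blackboard the airborne player's floor and retarget to damage causers; close-range montage attacks temporarily slow movement.
; Death awards XP, sometimes plays a sound and spawns any drop, while Tick turns the HP text toward the player.
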(event Custom|PlayerJumping
  (params (Floor :type Actor%20Object%20Reference))
  ;[1 1 1] BeginPlay
  (bind _output_get (Variables|Default|SetPlayerToFloor Floor))
  (Variables|Default|SetisPlayerInAir true)
  (AI|Components|Blackboard|SetValueasObject (AI|GetBlackboard 0) (Utilities|Name|MakeLiteralName "Floor") _output_get))

(event Custom|CheckDistance_Event
  ;[1 1 1] Locomotion check for Behaviour Tree
  (if (and (< (Math|Vector|Distance(Vector) (Transformation|GetActorLocation) (Transformation|GetActorLocation (Variables|Reference|GetTargetRef))) 2e+02) (Variables|Default|GetisAttackEnded))
    (CallFunction|Attack (Variables|Default|GetBaseAttackMontage) (Variables|Default|GetBaseAttackSound))))

(event Custom|PlayerGrounded
  ;[1 1 1] BeginPlay
  (bind _output_get (Variables|Default|SetPlayerToFloor 0))
  (Variables|Default|SetisPlayerInAir false)
  (AI|Components|Blackboard|SetValueasObject (AI|GetBlackboard 0) (Utilities|Name|MakeLiteralName "Floor") _output_get))

(event Custom|Attack
  (params (AnimMontage :type Anim%20Montage%20Object%20Reference) (AnimSound :type Sound%20Cue%20Object%20Reference))
  ;[1 1 1] Attack event + Play attack anim montage
  (Variables|Default|SetisAttackEnded false)
  (Variables|/Script/Engine.CharacterMovementComponent|SetMaxWalkSpeed (Variables|Character|GetCharacterMovement) 3.5e+02)
  (Audio|SpawnSoundAttached AnimSound (Variables|Collision|GetCapsuleComponent) "None" "0, 0, 0" "0, 0, 0" "KeepRelativeOffset" false 1.0 1.0 0.0 "/Game/Content/Sounds/SoundAttenuationSettings.SoundAttenuationSettings" 0)
  (bind _returnvalue (Animation|PlayAnimMontage AnimMontage 1.0 "None"))
  (Utilities|FlowControl|Delay _returnvalue)
  (Variables|/Script/Engine.CharacterMovementComponent|SetMaxWalkSpeed (Variables|Character|GetCharacterMovement) 6e+02)
  (Variables|Default|SetisAttackEnded true))

(event EventBeginPlay
  ;[1 1 1] BeginPlay
  (CallFunction|InitialSetup)
  (Variables|Character|Drop|SetDropRate (Math|Random|RandomFloatinRange 0.0 1e+02))
  (CallFunction|SetupDropRate))

(event EventCheckDistance
  ;[1 1 1] Locomotion check for Behaviour Tree
  (CallFunction|CheckDistanceEvent))

(event EventTick
  (params (DeltaSeconds :type Float%20%28single-precision%29))
  ;[1 1 1] Rotate Text renderer and print value
  (Transformation|SetWorldRotation (Variables|Default|GetHPRenderer) (Math|Rotator|FindLookatRotation (Transformation|GetWorldLocation (Variables|Default|GetHPRenderer)) (Transformation|GetActorLocation (Variables|Reference|GetPlayerRef))) false false)
  (Rendering|Components|TextRender|SetText (Variables|Default|GetELVRenderer) (Utilities|Text|ToText(Integer) (Math|Float|Truncate (Variables|Formula|GetELV)))))

(event EventTakeDamage
  (params (DamageReceived :type Float%20%28double-precision%29) (HitResult :type Hit%20Result%20Structure) (DamageCauser :type Actor%20Object%20Reference))
  ;[1 1 1] Damage Interface
  ;[1 1 1] change target after damage (if needed)
  (if (!= DamageCauser (Variables|Reference|GetTargetRef))
    (bind _output_get (Variables|Reference|SetTargetRef DamageCauser))
    (AI|SetFocus (AI|GetAIController self) _output_get)
    (AI|Components|Blackboard|SetValueasObject (AI|GetBlackboard 0) (Utilities|Name|MakeLiteralName "TargetRef") (Variables|Reference|GetTargetRef))))

(fn ConstructionScript)

(fn Death
  (CallFunction|XPReward)
  (if (< (Math|Random|RandomIntegerinRange 0 100) 21)
    (Audio|PlaySoundatLocation (Variables|Default|GetDeathSound) (Transformation|GetActorLocation) "0, 0, 0" 0.8 1.0 0.0 "/Game/Content/Sounds/SoundAttenuationSettings.SoundAttenuationSettings" 0 0 0))
  (CallFunction|SpawnDrop)
  (Actor|DestroyActor))

(fn SetupDropRate
  (if (<= (Variables|Character|Drop|GetDropRate) 9e+01)
    (return)
    (elif (and (> (Variables|Character|Drop|GetDropRate) 9e+01) (<= (Variables|Character|Drop|GetDropRate) 94.25))
      (Variables|Character|Drop|SetDropToSpawn "/Game/Content/Gameplay/PowerUp/PiedeLesto/PiedeLesto_BP.PiedeLesto_BP_C")
      (return)
      (elif (and (> (Variables|Character|Drop|GetDropRate) 94.25) (<= (Variables|Character|Drop|GetDropRate) 98.5))
        (Variables|Character|Drop|SetDropToSpawn "/Game/Content/Gameplay/PowerUp/BalzoDelConiglio/BalzoDelConiglio_BP.BalzoDelConiglio_BP_C")
        (return)
        (elif (and (> (Variables|Character|Drop|GetDropRate) 98.5) (<= (Variables|Character|Drop|GetDropRate) 99.5))
          (Variables|Character|Drop|SetDropToSpawn "/Game/Content/Gameplay/PowerUp/Berserk/Berserk_BP.Berserk_BP_C")
          (return)
          (else
            ;[1 1 1] BonusToken
            (if (> (Variables|Character|Drop|GetDropRate) 99.5)
              (Variables|Character|Drop|SetDropToSpawn "/Game/Content/Gameplay/PowerUp/BonusToken/BonusToken_BP.BonusToken_BP_C")
              (return)
              (else
                (return)))))))))

(fn SpawnDrop
  (bind _returnvalue (Math|Random|RandomIntegerinRange 6 8))
  (if (> (Variables|Character|Drop|GetDropRate) 9e+01)
    (Utilities|IsValid self
      (:Is%20Valid
        (Game|SpawnActorfromClass (Variables|Character|Drop|GetDropToSpawn) (Math|Transform|MakeTransform (Transformation|GetWorldLocation (Variables|Default|GetPowerUpSpawn)) "0, 0, 0" "1.000000,1.000000,1.000000") "AlwaysSpawn" 0 _returnvalue false (+ (Math|Conversions|ToFloat(Integer) _returnvalue) 5.0) 0 0)
        (return))
      (:Is%20Not%20Valid
        (Development|PrintString "Error" true true "(R=0.953000,G=0.000000,B=0.000000,A=1.000000)")))))

(fn InitialSetup
  (bind _masterspawnerref (Variables|Reference|GetMasterSpawnerRef))
  (for _index (range 1 (- (Math|Float|Truncate (Variables|Formula|GetELV)) (Variables|/Game/Content/Gameplay/Spawner/Spawner_MasterBP.Spawner_MasterBP_C|GetELVApplied (Variables|Reference|GetMasterSpawnerRef))))
    (Default|UpdateEnemyMapValue _masterspawnerref)
    (Variables|Character|Stats|SetHPMax (.Value (Utilities|Map|Find (Variables|/Game/Content/Gameplay/Spawner/Spawner_MasterBP.Spawner_MasterBP_C|GetActualEnemyHPMap _masterspawnerref) (Utilities|GetClass self)))))
  (Variables|/Game/Content/Gameplay/Spawner/Spawner_MasterBP.Spawner_MasterBP_C|SetELVApplied (Variables|Reference|GetMasterSpawnerRef) (Math|Float|Truncate (Variables|Formula|GetELV)))
  (Utilities|Map|Add (Variables|/Game/Content/Gameplay/Spawner/Spawner_MasterBP.Spawner_MasterBP_C|GetActualEnemyHPMap (Variables|Reference|GetMasterSpawnerRef)) (Utilities|GetClass self) (Variables|Character|Stats|GetHPMax))
  (bind _output_get (Variables|Character|Stats|SetHPCurrent (Math|Conversions|ToFloat(Integer) (Math|Float|Truncate (Variables|Character|Stats|GetHPMax)))))
  (Rendering|Components|TextRender|SetText (Variables|Default|GetHPRenderer) (Utilities|Text|ToText(Float) _output_get "HalfToEven")))

(fn XPReward
  (Default|PlayerLevelFunc (Variables|Reference|GetPlayerRef) (* (Variables|Formula|GetCD) (Variables|Formula|GetEnemyValue)))
  (return))