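; Tank enemy character that takes half damage unless the hit strikes its back collider, its weak spot.
; TakeDamage calls the parent, scales damage and applies it as point damage, which updates the HP text or notifies the master spawner and triggers death.
; Attack start/end events toggle punch collision, which sends damage to Player-tagged actors on overlap.
; The construction script binds modular limb, tail and head meshes to the main mesh's pose.
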(event OnComponentBeginOverlap(PunchCollision)
  (params (OverlappedComponent :type Primitive%20Component%20Object%20Reference) (OtherActor :type Actor%20Object%20Reference) (OtherComp :type Primitive%20Component%20Object%20Reference) (OtherBodyIndex :type Integer) (bFromSweep :type Boolean) (SweepResult :type Hit%20Result%20Structure%20%28by%20ref%29))
  (if (Actor|ActorHasTag OtherActor "Player")
    (Class|TakeDamageInterface|TakeDamage(Message) OtherActor (Variables|Default|GetDamage) SweepResult self)))

(event Custom|AttackDamageStart
  (Collision|SetCollisionEnabled (Variables|Default|GetPunchCollision) "QueryAndPhysics"))

(event Custom|AttackDamageEnd
  (Collision|SetCollisionEnabled (Variables|Default|GetPunchCollision) "NoCollision"))

(event Game|Damage|EventPointDamage
  (params (Damage :type Float%20%28single-precision%29) (DamageType :type Damage%20Type%20Object%20Reference) (HitLocation :type Vector :default "0, 0, 0") (HitNormal :type Vector :default "0, 0, 0") (HitComponent :type Primitive%20Component%20Object%20Reference) (BoneName :type Name :default "None") (ShotFromDirection :type Vector :default "0, 0, 0") (InstigatedBy :type Controller%20Object%20Reference) (DamageCauser :type Actor%20Object%20Reference) (HitInfo :type Hit%20Result%20Structure%20%28by%20ref%29))
  ;[0 1 0.1588] Damage Function (Interface)
  (if (> (- (Variables|Default|GetHPCurrent) Damage) 0.0)
    (bind _output_get (Variables|Default|SetHPCurrent (- (Variables|Default|GetHPCurrent) Damage)))
    (Rendering|Components|TextRender|SetText (Variables|Default|GetHPRenderer) (Utilities|Text|ToText(Float) _output_get "HalfToEven"))
    (else
      (Default|EnemyDied (Variables|Default|GetMasterSpawnerRef) (Variables|Default|GetIndex))
      (CallFunction|Death))))

(event EventTakeDamage
  (params (DamageReceived :type Float%20%28double-precision%29) (HitResult :type Hit%20Result%20Structure) (DamageCauser :type Actor%20Object%20Reference))
  (bind (_bblockinghit _binitialoverlap _time _distance _location _impactpoint _normal _impactnormal _physmat _hitactor _hitcomponent _hitbonename _bonename _hititem _elementindex _faceindex _tracestart) (Collision|BreakHitResult HitResult))
  ;[0 1 0.1588] TakeDamage Function
  (|CallParentFunction DamageReceived HitResult DamageCauser)
  (Variables|Default|SetDamageReceived DamageReceived)
  (if (== _hitcomponent (Variables|Default|GetBackDamageColl))
    _
    (else
      (Variables|Default|SetDamageReceived (* (Variables|Default|GetDamageReceived) 0.5))))
  (Game|Damage|ApplyPointDamage self (Variables|Default|GetDamageReceived) _tracestart HitResult 0 DamageCauser))

(fn ConstructionScript
  (|CallParentFunction)
  (for _array_element (Utilities|Array|MakeArray (Variables|Default|GetLeftArm) (Variables|Default|GetRightArm) (Variables|Default|GetLeftLeg) (Variables|Default|GetTail) (Variables|Default|GetRightLeg) (Variables|Default|GetHead))
    (Class|SkinnedMeshComponent|SetMasterPoseComponent _array_element (Variables|Character|GetMesh) false)))