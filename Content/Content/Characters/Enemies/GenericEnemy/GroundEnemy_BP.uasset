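; Ground enemy character with a modular body, health display and melee attack, reporting its death to a master spawner.
; Incoming hits get a headshot multiplier, then route through point damage to reduce HP or trigger death.
; AttackDamage sphere-traces at the right-hand socket and passes damage to the hit actor by message.
; The construction script makes limb, head and tail meshes follow the main mesh via master pose.
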(event Game|Damage|EventPointDamage
  (params (Damage :type Float%20%28single-precision%29) (DamageType :type Damage%20Type%20Object%20Reference) (HitLocation :type Vector :default "0, 0, 0") (HitNormal :type Vector :default "0, 0, 0") (HitComponent :type Primitive%20Component%20Object%20Reference) (BoneName :type Name :default "None") (ShotFromDirection :type Vector :default "0, 0, 0") (InstigatedBy :type Controller%20Object%20Reference) (DamageCauser :type Actor%20Object%20Reference) (HitInfo :type Hit%20Result%20Structure%20%28by%20ref%29))
  ;[0 1 0.1588] Damage Function (Interface)
  (if (> (- (Variables|Default|GetHPCurrent) Damage) 0.0)
    (bind _output_get (Variables|Default|SetHPCurrent (- (Variables|Default|GetHPCurrent) Damage)))
    (Rendering|Components|TextRender|SetText (Variables|Default|GetHPRenderer) (Utilities|Text|ToText(Float) _output_get "HalfToEven"))
    (else
      (Default|EnemyDied (Variables|Default|GetMasterSpawnerRef) (Variables|Default|GetIndex))
      (CallFunction|Death))))

(event EventTakeDamage
  (params (DamageReceived :type Float%20%28double-precision%29) (HitResult :type Hit%20Result%20Structure) (DamageCauser :type Actor%20Object%20Reference))
  (bind (_bblockinghit _binitialoverlap _time _distance _location _impactpoint _normal _impactnormal _physmat _hitactor _hitcomponent _hitbonename _bonename _hititem _elementindex _faceindex _tracestart) (Collision|BreakHitResult HitResult))
  ;[0 1 0.1588] TakeDamage Function
  (|CallParentFunction DamageReceived HitResult DamageCauser)
  (Variables|Default|SetDamageReceived DamageReceived)
  (if (!= _hitbonename "head")
    _
    (else
      (Variables|Default|SetDamageReceived (* (Variables|Default|GetDamageReceived) 4.0))))
  (Game|Damage|ApplyPointDamage self (Variables|Default|GetDamageReceived) _tracestart HitResult 0 DamageCauser))

(fn ConstructionScript
  (|CallParentFunction)
  (for _array_element (Utilities|Array|MakeArray (Variables|Default|GetLeftArm) (Variables|Default|GetRightArm) (Variables|Default|GetLeftLeg) (Variables|Default|GetTail) (Variables|Default|GetRightLeg) (Variables|Default|GetHead))
    (Class|SkinnedMeshComponent|SetMasterPoseComponent _array_element (Variables|Character|GetMesh) false)))

(fn AttackDamage
  (bind _rhandsocket (Variables|Default|GetRHandSocket))
  (bind _returnvalue (Transformation|GetWorldLocation _rhandsocket))
  (bind (_outhit _returnvalue_2) (Collision|SphereTraceByChannel _returnvalue _returnvalue 1.5e+02 "TraceTypeQuery5" false 0 "None"))
  (if _returnvalue_2
    (Class|TakeDamageInterface|TakeDamage(Message) (.HitActor (Collision|BreakHitResult _outhit)) (Variables|Default|GetDamage) _outhit self)))