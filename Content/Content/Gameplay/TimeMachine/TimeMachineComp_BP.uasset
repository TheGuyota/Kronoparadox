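; TimeMachineComp_BP is a collectible time machine component that the player picks up by walking into it.
; Each tick, its Cube rotates to face the player character.
; When a Player-tagged MainCharacter_BP overlaps Sphere1 while holding fewer than three components, it increments that character's count, updates the in-game UI and destroys itself.
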(event OnComponentBeginOverlap(Sphere1)
  (params (OverlappedComponent :type Primitive%20Component%20Object%20Reference) (OtherActor :type Actor%20Object%20Reference) (OtherComp :type Primitive%20Component%20Object%20Reference) (OtherBodyIndex :type Integer) (bFromSweep :type Boolean) (SweepResult :type Hit%20Result%20Structure%20%28by%20ref%29))
  (bind _asmain_character_bp (Utilities|Casting|CastToMainCharacter_BP OtherActor))
  (bind _timemachinecomponents (Variables|/Game/Content/Characters/Player/MainCharacter_BP.MainCharacter_BP_C|GetTimeMachineComponents _asmain_character_bp))
  (if (Actor|ActorHasTag OtherActor "Player")
    (Utilities|IsValid _asmain_character_bp
      (:Is%20Valid
        (if (< _timemachinecomponents 3)
          (Math|Integer|IncrementInt _timemachinecomponents
            (:%20%20
              (Default|UpdateTimeMachineComponent (Variables|/Game/Content/Characters/Player/MainCharacter_BP.MainCharacter_BP_C|GetInGameUI _asmain_character_bp) true)
              (Actor|DestroyActor))))))))

(event EventTick
  (params (DeltaSeconds :type Float%20%28single-precision%29))
  (Transformation|SetWorldRotation (Variables|Default|GetCube) (Math|Rotator|FindLookatRotation (Transformation|GetWorldLocation (Variables|Default|GetCube)) (Transformation|GetActorLocation (Game|GetPlayerCharacter 0))) false false))

(fn ConstructionScript)