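; Time machine actor the player must keep alive: it tracks HP, takes damage and triggers game over on the player when HP reaches zero.
; While the player overlaps its box, a looping timer spends carried components to restore HP and update the UI.
; Leaving the box or non-lethal damage clears that repair timer.
; A second timer keeps the floating HP text turned toward the player.
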(event OnComponentBeginOverlap(Box)
  (params (OverlappedComponent :type Primitive%20Component%20Object%20Reference) (OtherActor :type Actor%20Object%20Reference) (OtherComp :type Primitive%20Component%20Object%20Reference) (OtherBodyIndex :type Integer) (bFromSweep :type Boolean) (SweepResult :type Hit%20Result%20Structure%20%28by%20ref%29))
  (if (== OtherActor (Variables|Default|GetPlayerRef))
    (Variables|Default|SetActorInRange OtherActor)
    (bind _returnvalue (Utilities|Time|SetTimerbyEvent (EventDispatchers|CreateEvent :!event Custom|AddMachineComponent) 1.5 true))
    (Variables|Default|SetAddMachineComponentHandle _returnvalue)))

(event OnComponentEndOverlap(Box)
  (params (OverlappedComponent :type Primitive%20Component%20Object%20Reference) (OtherActor :type Actor%20Object%20Reference) (OtherComp :type Primitive%20Component%20Object%20Reference) (OtherBodyIndex :type Integer))
  (if (== OtherActor (Variables|Default|GetPlayerRef))
    (Variables|Default|SetActorInRange 0)
    (Utilities|Time|ClearandInvalidateTimerbyHandle (Variables|Default|GetAddMachineComponentHandle))))

(event Custom|RotateHPRenderer
  ;[1 1 1] BeginPlay + Update Rotation
  (Transformation|SetWorldRotation (Variables|Default|GetHP) (Math|Rotator|FindLookatRotation (Transformation|GetWorldLocation (Variables|Default|GetHP)) (Transformation|GetActorLocation (Variables|Default|GetPlayerRef))) false false))

(event Custom|AddMachineComponent
  (bind _playerref (Variables|Default|GetPlayerRef))
  (bind _timemachinecomponents (Variables|/Game/Content/Characters/Player/MainCharacter_BP.MainCharacter_BP_C|GetTimeMachineComponents _playerref))
  (Variables|Default|GetActorInRange
    (:then
      (if (and (> _timemachinecomponents 0) (< (Variables|Default|GetHPActual) (Variables|Default|GetHPMax)))
        (Math|Integer|DecrementInt _timemachinecomponents
          (:%20%20
            (bind _output_get (Variables|Default|SetHPActual (Math|Float|Clamp(Float) (+ (Variables|Default|GetHPActual) 2.5e+02) 0.0 1e+03)))
            (Rendering|Components|TextRender|SetText (Variables|Default|GetHP) (Utilities|Text|ToText(Float) _output_get "HalfToEven"))
            (Default|UpdateTimeMachineComponent (Variables|/Game/Content/Characters/Player/MainCharacter_BP.MainCharacter_BP_C|GetInGameUI (Variables|Default|GetPlayerRef)) false)))
        (else
          (Utilities|Time|ClearandInvalidateTimerbyHandle (Variables|Default|GetAddMachineComponentHandle)))))
    (:else)))

(event EventTakeDamage
  (params (DamageReceived :type Float%20%28double-precision%29) (HitResult :type Hit%20Result%20Structure) (DamageCauser :type Actor%20Object%20Reference))
  ;[1 1 1] TakeDamage
  (if (> (- (Variables|Default|GetHPActual) DamageReceived) 0.0)
    (bind _output_get (Variables|Default|SetHPActual (- (Variables|Default|GetHPActual) DamageReceived)))
    (Rendering|Components|TextRender|SetText (Variables|Default|GetHP) (Utilities|Text|ToText(Float) _output_get "HalfToEven"))
    (Utilities|Time|ClearandInvalidateTimerbyHandle (Variables|Default|GetAddMachineComponentHandle))
    (else
      (bind _output_get_2 (Variables|Default|SetHPActual 0.0))
      (Rendering|Components|TextRender|SetText (Variables|Default|GetHP) (Utilities|Text|ToText(Float) _output_get_2 "HalfToEven"))
      (Default|PlayerGameOver (Variables|Default|GetPlayerRef)))))

(event EventBeginPlay
  ;[1 1 1] BeginPlay + Update Rotation
  (bind _returnvalue (Actor|GetActorOfClass "/Game/Content/Characters/Player/MainCharacter_BP.MainCharacter_BP_C"))
  (Variables|Default|SetPlayerRef _returnvalue)
  (Utilities|Time|SetTimerbyEvent (delegate Custom|RotateHPRenderer) 0.1 true))

(fn ConstructionScript
  (bind _output_get (Variables|Default|SetHPActual (Variables|Default|GetHPMax)))
  (Rendering|Components|TextRender|SetText (Variables|Default|GetHP) (Utilities|Text|ToText(Float) _output_get "HalfToEven")))