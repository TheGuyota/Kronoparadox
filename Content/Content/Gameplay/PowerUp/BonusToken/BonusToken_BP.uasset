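; BonusToken_BP is a pickup actor that grants the player a bonus token.
; When an actor tagged Player overlaps its Box, it casts to MainCharacter_BP and checks whether a token is already held.
; If none is held, it sets the character's BonusToken flag, shows the token in the in-game UI and destroys itself, so only one token is carried at once.
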(event OnComponentBeginOverlap(Box)
  (params (OverlappedComponent :type Primitive%20Component%20Object%20Reference) (OtherActor :type Actor%20Object%20Reference) (OtherComp :type Primitive%20Component%20Object%20Reference) (OtherBodyIndex :type Integer) (bFromSweep :type Boolean) (SweepResult :type Hit%20Result%20Structure%20%28by%20ref%29))
  (if (Actor|ActorHasTag OtherActor "Player")
    (bind _output_get (Variables|Default|SetMainCharacterRef (.AsMain%20Character%20BP (Utilities|Casting|CastToMainCharacter_BP OtherActor))))
    (if (not (Variables|/Game/Content/Characters/Player/MainCharacter_BP.MainCharacter_BP_C|GetBonusToken _output_get))
      (Variables|/Game/Content/Characters/Player/MainCharacter_BP.MainCharacter_BP_C|SetBonusToken (Variables|Default|GetMainCharacterRef) true)
      (Default|UpdateBonusTokenVisibility (Variables|/Game/Content/Characters/Player/MainCharacter_BP.MainCharacter_BP_C|GetInGameUI (Variables|Default|GetMainCharacterRef)) true)
      (Actor|DestroyActor))))

(fn ConstructionScript
  (|CallParentFunction))