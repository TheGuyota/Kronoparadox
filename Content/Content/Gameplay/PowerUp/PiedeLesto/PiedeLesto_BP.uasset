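; Speed power-up pickup (PiedeLesto) that temporarily changes the player's max walk speed when overlapped.
; On overlap it destroys the player's current non-static PiedeLesto, passes itself to the character to apply the effect, then starts a countdown and expiry timer.
; On expiry, only the still-current pickup restores walk speed and footstep interval to hard-coded values and clears itself, limiting stacking.
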(event OnComponentBeginOverlap(Box)
  (params (OverlappedComponent :type Primitive%20Component%20Object%20Reference) (OtherActor :type Actor%20Object%20Reference) (OtherComp :type Primitive%20Component%20Object%20Reference) (OtherBodyIndex :type Integer) (bFromSweep :type Boolean) (SweepResult :type Hit%20Result%20Structure%20%28by%20ref%29))
  ;[1 1 1] If player overlap update max velocity -with some stack limitation-
  (if (Actor|ActorHasTag OtherActor "Player")
    (Variables|Default|SetCountdown (Variables|Default|GetPowerUpDuration))
    (bind _output_get (Variables|Default|SetMainCharacterRef (.AsMain%20Character%20BP (Utilities|Casting|CastToMainCharacter_BP OtherActor))))
    (bind _current_piedelesto (Variables|/Game/Content/Characters/Player/MainCharacter_BP.MainCharacter_BP_C|GetCurrent_PiedeLesto _output_get)
      (:then
        (if (Variables|/Game/Content/Gameplay/PowerUp/PowerUp_MasterBP.PowerUp_MasterBP_C|GetisStatic _current_piedelesto)
          _
          (else
            (Actor|DestroyActor _current_piedelesto))))
      (:else
        _))
    (Default|PowerUpPiedeLesto (Variables|Default|GetMainCharacterRef) self)
    (Audio|PlaySoundatLocation "/Game/Content/Sounds/Feedback/Power_Up/PowerUp_Generico.PowerUp_Generico" (Transformation|GetActorLocation) "0, 0, 0" 1.0 1.0 0.0 0 0 0 0)
    (Utilities|Time|SetTimerbyEvent (delegate Custom|StopPowerUp) (Math|Conversions|ToFloat(Integer) (Variables|Default|GetPowerUpDuration)))
    (CallFunction|CountdownandStaticCheck)))

(event Custom|StopPowerUp
  ;[1 1 1] If player overlap update max velocity -with some stack limitation-
  (if (== (Variables|/Game/Content/Characters/Player/MainCharacter_BP.MainCharacter_BP_C|GetCurrent_PiedeLesto (Variables|Default|GetMainCharacterRef)) self)
    (Variables|/Script/Engine.CharacterMovementComponent|SetMaxWalkSpeed (Variables|/Script/Engine.Character|GetCharacterMovement (Variables|Default|GetMainCharacterRef)) 1.05e+03)
    (Variables|/Game/Content/Characters/Player/MainCharacter_BP.MainCharacter_BP_C|SetFootstepInterval (Variables|Default|GetMainCharacterRef) 0.25)
    (Default|ResetFootstep (Variables|Default|GetMainCharacterRef))
    (Variables|/Game/Content/Characters/Player/MainCharacter_BP.MainCharacter_BP_C|SetCurrent_PiedeLesto (Variables|Default|GetMainCharacterRef) 0)
    (Audio|PlaySound2D "/Game/Content/Sounds/Feedback/Power_Up/Power_Up_svanisce.Power_Up_svanisce" 1.0 1.0 0.0 0 0)
    (Utilities|Time|ClearandInvalidateTimerbyHandle (Variables|Default|GetCountDownHandle))))

(fn ConstructionScript
  (|CallParentFunction))