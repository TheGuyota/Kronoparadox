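; BalzoDelConiglio_BP is a jump power-up pickup, activated when an actor tagged Player overlaps its box.
; It replaces the character's current instance, destroying it unless static, then passes itself to the character's PowerUpBalzoDelConiglio and runs CountdownAndStaticCheck.
; A timer ends the effect, restoring default jump velocity and clearing the countdown only if this instance is still the active one.
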(event OnComponentBeginOverlap(Box)
  (params (OverlappedComponent :type Primitive%20Component%20Object%20Reference) (OtherActor :type Actor%20Object%20Reference) (OtherComp :type Primitive%20Component%20Object%20Reference) (OtherBodyIndex :type Integer) (bFromSweep :type Boolean) (SweepResult :type Hit%20Result%20Structure%20%28by%20ref%29))
  (if (Actor|ActorHasTag OtherActor "Player")
    (Variables|Default|SetCountdown (Variables|Default|GetPowerUpDuration))
    (bind _output_get (Variables|Default|SetMainCharacterRef (.AsMain%20Character%20BP (Utilities|Casting|CastToMainCharacter_BP OtherActor))))
    (bind _current_balzodelconiglio (Variables|/Game/Content/Characters/Player/MainCharacter_BP.MainCharacter_BP_C|GetCurrent_BalzoDelConiglio _output_get)
      (:then
        (if (Variables|/Game/Content/Gameplay/PowerUp/PowerUp_MasterBP.PowerUp_MasterBP_C|GetisStatic _current_balzodelconiglio)
          _
          (else
            (Actor|DestroyActor _current_balzodelconiglio))))
      (:else
        _))
    (Default|PowerUpBalzoDelConiglio (Variables|Default|GetMainCharacterRef) self)
    (Utilities|Time|SetTimerbyEvent (delegate Custom|StopPowerUp) (Math|Conversions|ToFloat(Integer) (Variables|Default|GetPowerUpDuration)))
    (CallFunction|CountdownandStaticCheck)))

(event Custom|StopPowerUp
  (if (== (Variables|/Game/Content/Characters/Player/MainCharacter_BP.MainCharacter_BP_C|GetCurrent_BalzoDelConiglio (Variables|Default|GetMainCharacterRef)) self)
    (Variables|/Script/Engine.CharacterMovementComponent|SetJumpZVelocity (Variables|/Script/Engine.Character|GetCharacterMovement (Variables|Default|GetMainCharacterRef)) 4.2e+02)
    (Variables|/Game/Content/Characters/Player/MainCharacter_BP.MainCharacter_BP_C|SetCurrent_BalzoDelConiglio (Variables|Default|GetMainCharacterRef) 0)
    (Utilities|Time|ClearandInvalidateTimerbyHandle (Variables|Default|GetCountDownHandle))))

(fn ConstructionScript
  (|CallParentFunction))