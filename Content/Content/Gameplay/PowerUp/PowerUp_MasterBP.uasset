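; Base power-up Blueprint that spins continuously in the world and either respawns or is destroyed after use.
; A looping timer drives the rotation from BeginPlay.
; CountdownAndStaticCheck hides the actor, disables its box collision, and starts both a per-second countdown and a respawn delay.
; When the delay ends, static power-ups reappear with collision restored, while others destroy themselves.
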(event Custom|RespawnOrDestroy
  (if (Variables|Default|GetisStatic)
    (Rendering|SetActorHiddenInGame self false)
    (Collision|SetCollisionEnabled (Variables|Default|GetBox) "QueryAndPhysics")
    (else
      (Actor|DestroyActor))))

(event Custom|CountdownAndStaticCheck
  (bind _returnvalue (Utilities|Time|SetTimerbyEvent (delegate Custom|CountdownFunc) 1.0 true))
  (Variables|Default|SetCountDownHandle _returnvalue)
  (Rendering|SetActorHiddenInGame self true)
  (Collision|SetCollisionEnabled (Variables|Default|GetBox) "NoCollision")
  (Utilities|Time|SetTimerbyEvent (delegate Custom|RespawnOrDestroy) (Variables|Default|GetSecondsBetweenRespawn)))

(event Custom|CountdownFunc
  (Math|Integer|DecrementInt (Variables|Default|GetCountdown)))

(event Custom|RotateMesh
  (Class|Actor|AddActorWorldRotation self "0,2.000000, 0"))

(event EventBeginPlay
  (Utilities|Time|SetTimerbyEvent (delegate Custom|RotateMesh) 0.03 true))

(fn ConstructionScript)