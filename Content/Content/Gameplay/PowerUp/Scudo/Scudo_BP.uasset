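; Shield power-up pickup that restores shield to the player on overlap.
; When an actor tagged Player enters the box, it casts to MainCharacter_BP and acts only if the current shield differs from the maximum.
; It then plays the Scudo sound at its location, passes ShieldAmount to the character's ShieldManagement and calls CountdownAndStaticCheck.
; The construction script only runs the parent's version.
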(event OnComponentBeginOverlap(Box)
  (params (OverlappedComponent :type Primitive%20Component%20Object%20Reference) (OtherActor :type Actor%20Object%20Reference) (OtherComp :type Primitive%20Component%20Object%20Reference) (OtherBodyIndex :type Integer) (bFromSweep :type Boolean) (SweepResult :type Hit%20Result%20Structure%20%28by%20ref%29))
  ;[1 1 1] If player overlap with shield powerup update the amount
  (if (Actor|ActorHasTag OtherActor "Player")
    (bind _output_get (Variables|Default|SetMainCharacterRef (.AsMain%20Character%20BP (Utilities|Casting|CastToMainCharacter_BP OtherActor))))
    (if (not (== (Variables|/Game/Content/Characters/Player/MainCharacter_BP.MainCharacter_BP_C|GetShieldCurrent _output_get) (Variables|/Game/Content/Characters/Player/MainCharacter_BP.MainCharacter_BP_C|GetShieldMax (Variables|Default|GetMainCharacterRef))))
      (Audio|PlaySoundatLocation "/Game/Content/Sounds/Feedback/Power_Up/Scudo.Scudo" (Transformation|GetActorLocation) "0, 0, 0" 1.0 1.0 0.0 0 0 0 0)
      (Default|ShieldManagement _output_get (Variables|Default|GetShieldAmount))
      (CallFunction|CountdownandStaticCheck))))

(fn ConstructionScript
  (|CallParentFunction))