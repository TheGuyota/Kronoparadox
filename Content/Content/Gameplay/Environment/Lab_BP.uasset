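; Lab_BP is an environment actor that shows one of several lab map variants through a child actor and changes it on time travel.
; The construction script assigns a random class from MapVariants.
; On BeginPlay it registers TimeTravel with the StandardGameMode time travel dispatcher.
; TimeTravel rerolls GetRandomEra until the result differs from the current era, then swaps the child actor class.
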(event Custom|TimeTravel
  (Variables|Default|SetLastEra (Variables|/Script/Engine.ChildActorComponent|GetChildActorClass (Variables|Default|GetChildActor)))
  (bind _randomizedera (CallFunction|GetRandomEra :!label _label))
  (if (!= _randomizedera (Variables|Default|GetLastEra))
    (ChildActorComponent|SetChildActorClass (Variables|Default|GetChildActor) _randomizedera)
    (else
      (goto _label))))

(event EventBeginPlay
  (bind _asstandard_game_mode (Utilities|Casting|CastToStandardGameMode (Game|GetGameMode)))
  (EventDispatchers|BindEventtoTimeTravelDispatcher _asstandard_game_mode (delegate Custom|TimeTravel)))

(fn ConstructionScript
  (ChildActorComponent|SetChildActorClass (Variables|Default|GetChildActor) (.OutItem (Utilities|Array|Random (Variables|Default|GetMapVariants)))))

(fn GetRandomEra
  (return (.OutItem (Utilities|Array|Random (Variables|Default|GetMapVariants)))))