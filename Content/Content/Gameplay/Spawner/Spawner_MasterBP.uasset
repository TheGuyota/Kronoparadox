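; Wave manager that spawns enemies at random EnemySpawner_BP actors and periodically places time machine components.
; Looping timers drive growing normal waves and recurring timed special waves targeting the time machine, with enemy types weighted by wave section.
; A difficulty coefficient, exponential in completed stages and recalculated on time travel, sets enemy level.
; Enemy deaths trigger the next wave, a delayed check destroys stuck last enemies, and completed waves can be sent to PlayFab.
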(event Custom|CheckForMachineComponent
  ;[1 1 1] Spawn Time Machine Component
  (Variables|TimeMachine|Components|GetActualSpawnedComponent
    (:then
      (Variables|TimeMachine|Components|SetMachineComponentCounter 0))
    (:else
      (bind _result (Math|Integer|IncrementInt (Variables|TimeMachine|Components|GetMachineComponentCounter))
        (:%20%20
          (if (== _result (Variables|TimeMachine|Components|GetWaveBetweenComponentSpawn))
            (bind _actualcomponent (Default|SpawnComponent (.OutItem (Utilities|Array|Random (Variables|TimeMachine|Components|GetMachineComponentSpawners)))))
            (Variables|TimeMachine|Components|SetActualSpawnedComponent _actualcomponent)
            (Variables|TimeMachine|Components|SetMachineComponentCounter 0)))))))

(event Custom|StartEnemyWave
  ;[1 1 1] Enemy Wave System
  (CallFunction|StartLastEnemiesCheck)
  (bind _result (Math|Integer|IncrementInt (Variables|WaveInfo|GetWaveCounter))
    (:%20%20
      (Default|CallUpdateWaveCounter _result)
      (Variables|Formula|Raw|SetCompletedStages (- _result 1))
      (CallFunction|UpdateWaveSection)
      (CallFunction|CheckforMachineComponent)
      (if (!= (Variables|WaveInfo|GetWaveCounter) (Variables|SpecialWave|GetSpecialWaveMultiplier))
        (bind _returnvalue (Utilities|Time|SetTimerbyFunctionName 0 "NormalWave" 1.0 true))
        (Variables|EnemySpawner|Other|SetNormalWaveSpawnerHandle _returnvalue)
        (else
          (Variables|SpecialWave|SetActualSpecialWaveTimer (Variables|SpecialWave|GetSpecialWaveTimeLimit))
          (Default|PlaySpecialWave (Variables|/Game/Content/Characters/Player/MainCharacter_BP.MainCharacter_BP_C|GetInGameUI (Variables|Ref|GetPlayerRef)))
          (for _array_element (Variables|EnemySpawner|Other|GetEnemySpawners)
            (CallFunction|SpawnSingleRandomEnemySpecialWave _array_element))
          (bind _returnvalue_2 (Utilities|Time|SetTimerbyFunctionName 0 "SpecialWave" 1.0 true 1.0))
          (Variables|SpecialWave|SetSpecialWaveSpawnerHandle _returnvalue_2)
          (bind _returnvalue_3 (Utilities|Time|SetTimerbyEvent (delegate Custom|SpecialWaveTimer) 1.0 true)))))))

(event Custom|EnemyDied
  (params (EnemyIndex :type Integer))
  ;[1 1 1] Remove the first elementh of the array when an enemy die
  (Utilities|Array|RemoveIndex (Variables|EnemySpawner|Other|GetEnemiesSpawned))
  (if (and (== (Utilities|Array|Length (Variables|EnemySpawner|Other|GetEnemiesSpawned)) 0) (Variables|Default|GetAllEnemySpawned))
    (Utilities|FlowControl|Delay (Variables|WaveInfo|GetTimeBetweenEachWave))
    (CallFunction|StartEnemyWave)))

(event Custom|SpecialWaveTimer
  ;[1 1 1] Enemy Wave System
  (bind _result (Math|Integer|DecrementInt (Variables|SpecialWave|GetActualSpecialWaveTimer))
    (:%20%20
      (if (== _result 0)
        (Utilities|Time|ClearandInvalidateTimerbyHandle (stale Custom|StartEnemyWave _returnvalue_3))))))

(event Custom|SendWaveCounterToPlayfab
  ;[1 1 1] PLAYFAB
  (Default|SendWaveSurpassed (Variables|Ref|GetGameInstanceRef) (Variables|Formula|Raw|GetCompletedStages)))

(event Custom|CheckCoefficente
  ;[1 0 0.765] Formula di un noto matematico
  (Math|Float|IncrementFloat (Variables|Formula|Raw|GetTimeInt)
    (:%20%20
      (bind _cd (CallFunction|CoefficenteDifficolta))
      (CallFunction|EnemyLevel _cd))))

(event Custom|CheckForEnemyStuck
  ;[1 1 1] Destroy the last 2 (or less) enemies alive after 20 seconds
  (if (and (<= (Utilities|Array|Length (Variables|EnemySpawner|Other|GetEnemiesSpawned)) 2) (> (Utilities|Array|Length (Variables|EnemySpawner|Other|GetEnemiesSpawned)) 0))
    (Variables|Default|SetActualWaveToApplyFix (Variables|WaveInfo|GetWaveCounter))
    (Development|PrintString "2 or less enemy found")
    (Utilities|Time|ClearandInvalidateTimerbyHandle (Variables|Default|GetCheckForEnemy))
    (Utilities|Time|SetTimerbyEvent (delegate Custom|DestroyStuckEnemy) 2e+01)))

(event Custom|DestroyStuckEnemy
  ;[1 1 1] Destroy the last 2 (or less) enemies alive after 20 seconds
  (if (== (Variables|Default|GetActualWaveToApplyFix) (Variables|WaveInfo|GetWaveCounter))
    (bind _outactors (Actor|GetAllActorsOfClass "/Game/Content/Characters/Enemies/Enemy_MasterBP.Enemy_MasterBP_C"))
    (for _array_element _outactors
      (CallFunction|EnemyDied)
      (Actor|DestroyActor _array_element))
    (Development|PrintString "Enemies Exploded")
    (else
      (Variables|Default|SetActualWaveToApplyFix 0))))

(event Custom|StartLastEnemiesCheck
  ;[1 1 1] Destroy the last 2 (or less) enemies alive after 20 seconds
  (bind _returnvalue (Utilities|Time|SetTimerbyEvent (delegate Custom|CheckForEnemyStuck) 15.0 true))
  (Variables|Default|SetCheckForEnemy _returnvalue))

(event EventBeginPlay
  ;[1 1 1] BeginPlay
  (Utilities|FlowControl|Sequence
    (:then_0
      (bind _returnvalue (Actor|GetActorOfClass "/Game/Content/Characters/Player/MainCharacter_BP.MainCharacter_BP_C"))
      (bind _output_get (Variables|Ref|SetPlayerRef _returnvalue))
      (EventDispatchers|BindEventtoOnGameOver _output_get (EventDispatchers|CreateEvent :!event Custom|SendWaveCounterToPlayfab))
      (bind _outactors (Actor|GetAllActorsOfClass "/Game/Content/Gameplay/Spawner/EnemySpawner/EnemySpawner_BP.EnemySpawner_BP_C"))
      (Variables|EnemySpawner|Other|SetEnemySpawners _outactors)
      (bind _returnvalue_2 (Actor|GetActorOfClass "/Game/Content/Gameplay/TimeMachine/TimeMachine_BP.TimeMachine_BP_C"))
      (Variables|Ref|SetTimeMachineRef _returnvalue_2)
      (bind _asmain_game_instance (Utilities|Casting|CastToMainGameInstance (Game|GetGameInstance)))
      (Variables|Ref|SetGameInstanceRef _asmain_game_instance)
      (CallFunction|StartEnemyWave)
      (bind _outactors_2 (Actor|GetAllActorsOfClass "/Game/Content/Gameplay/TimeMachine/TimeMachineCompSpawn_BP.TimeMachineCompSpawn_BP_C"))
      (Variables|TimeMachine|Components|SetMachineComponentSpawners _outactors_2)
      (bind _asstandard_game_mode (Utilities|Casting|CastToStandardGameMode (Game|GetGameMode)))
      (EventDispatchers|BindEventtoTimeTravelDispatcher _asstandard_game_mode (delegate Custom|CheckCoefficente))
      (bind _cd (CallFunction|CoefficenteDifficolta))
      (CallFunction|EnemyLevel _cd))))

(event EventTick
  (params (DeltaSeconds :type Float%20%28single-precision%29))
  ;[1 0.8689 0.08085] Event TICK
  (if (!= (Variables|WaveInfo|GetWaveCounter) (Variables|SpecialWave|GetSpecialWaveMultiplier))
    (Development|PrintString (Utilities|String|Append "Wave N: " (Utilities|String|ToString(Integer) (Variables|WaveInfo|GetWaveCounter))) true true "(R=0.000000,G=0.660000,B=1.000000,A=1.000000)" 0.0)
    (Development|PrintString (Utilities|String|Append "Wave Between Component: " (Utilities|String|ToString(Integer) (Variables|TimeMachine|Components|GetMachineComponentCounter))) true true "(R=0.000000,G=0.660000,B=1.000000,A=1.000000)" 0.0)
    (Development|PrintString (Utilities|String|Append "Coefficente Difficoltà : " (Utilities|String|ToString(Float) (Variables|Formula|Calc|GetCoeffDiff))) true true "(R=0.000000,G=0.660000,B=1.000000,A=1.000000)" 0.0)
    (Development|PrintString (Utilities|String|Append "Livello Nemici : " (Utilities|String|ToString(Float) (Variables|Formula|Calc|GetActualEnemyLevel))) true true "(R=0.000000,G=0.660000,B=1.000000,A=1.000000)" 0.0)
    (Development|PrintString (Utilities|String|Append "Nemici vivi : " (Utilities|String|ToString(Integer) (Utilities|Array|Length (Variables|EnemySpawner|Other|GetEnemiesSpawned)))) true true "(R=1.000000,G=0.755457,B=0.000000,A=1.000000)" 0.0)
    (else
      (Development|PrintString "Special Wave" true true "(R=0.000000,G=0.660000,B=1.000000,A=1.000000)" 0.0)
      (Development|PrintString (Utilities|String|Append "Special Wave Timer : " (Utilities|String|ToString(Integer) (Variables|SpecialWave|GetActualSpecialWaveTimer))) true true "(R=0.000000,G=0.660000,B=1.000000,A=1.000000)" 0.0))))

(fn ConstructionScript)

(fn ChooseEnemytoSpawn
  (bind _enemytospawn (CallFunction|GetRightEnemytoSpawn))
  (Variables|EnemySpawner|Other|SetEnemyToSpawnClass _enemytospawn)
  (return))

(fn GetRightEnemytoSpawn
  (LocalVariables|SetRandomValue (Math|Random|RandomIntegerinRange 0 100))
  (switch Utilities|FlowControl|Switch|SwitchonWave_Enum (Variables|WaveInfo|GetActualWaveSection)
    (:NewEnumerator0
      (return "/Game/Content/Characters/Enemies/GenericEnemy/GroundEnemy_BP.GroundEnemy_BP_C"))
    (:NewEnumerator1
      (if (<= (LocalVariables|GetRandomValue) 90)
        (return "/Game/Content/Characters/Enemies/GenericEnemy/GroundEnemy_BP.GroundEnemy_BP_C")
        (elif (<= (LocalVariables|GetRandomValue) 92)
          (return "/Game/Content/Characters/Enemies/TankEnemy/TankEnemy_BP.TankEnemy_BP_C")
          (elif (<= (LocalVariables|GetRandomValue) 98)
            (return "/Game/Content/Characters/Enemies/GenericEnemy/GroundEnemy_BP.GroundEnemy_BP_C")
            (else
              (return "/Game/Content/Characters/Enemies/TankEnemy/TankEnemy_BP.TankEnemy_BP_C"))))))
    (:NewEnumerator2
      (if (<= (LocalVariables|GetRandomValue) 80)
        (return "/Game/Content/Characters/Enemies/GenericEnemy/GroundEnemy_BP.GroundEnemy_BP_C")
        (elif (<= (LocalVariables|GetRandomValue) 84)
          (return "/Game/Content/Characters/Enemies/TankEnemy/TankEnemy_BP.TankEnemy_BP_C")
          (elif (<= (LocalVariables|GetRandomValue) 96)
            (return "/Game/Content/Characters/Enemies/GenericEnemy/GroundEnemy_BP.GroundEnemy_BP_C")
            (else
              (return "/Game/Content/Characters/Enemies/TankEnemy/TankEnemy_BP.TankEnemy_BP_C"))))))
    (:NewEnumerator3
      (if (<= (LocalVariables|GetRandomValue) 65)
        (return "/Game/Content/Characters/Enemies/GenericEnemy/GroundEnemy_BP.GroundEnemy_BP_C")
        (elif (<= (LocalVariables|GetRandomValue) 75)
          (return "/Game/Content/Characters/Enemies/TankEnemy/TankEnemy_BP.TankEnemy_BP_C")
          (elif (<= (LocalVariables|GetRandomValue) 90)
            (return "/Game/Content/Characters/Enemies/GenericEnemy/GroundEnemy_BP.GroundEnemy_BP_C")
            (else
              (return "/Game/Content/Characters/Enemies/TankEnemy/TankEnemy_BP.TankEnemy_BP_C"))))))))

(fn UpdateWaveSection
  (if (< (Variables|WaveInfo|GetWaveCounter) 6)
    (return)
    (else
      (if (< (Variables|WaveInfo|GetWaveCounter) 11)
        (Variables|WaveInfo|SetActualWaveSection "NewEnumerator1")
        (elif (< (Variables|WaveInfo|GetWaveCounter) 16)
          (Variables|WaveInfo|SetActualWaveSection "NewEnumerator2")
          (else
            (Variables|WaveInfo|SetActualWaveSection "NewEnumerator3"))))
      (return))))

(fn NormalWave
  (bind _enemytospawnclass (Variables|EnemySpawner|Other|GetEnemyToSpawnClass))
  (bind _playerref (Variables|Ref|GetPlayerRef))
  (if (!= (Variables|NormalWave|GetEnemiesToSpawn) (Variables|EnemySpawner|Other|GetEnemySpawned))
    (Variables|Default|SetAllEnemySpawned false)
    (CallFunction|ChooseEnemytoSpawn)
    (bind _enemyspawned (Default|SpawnEnemy (.OutItem (Utilities|Array|Random (Variables|EnemySpawner|Other|GetEnemySpawners))) _enemytospawnclass (.Value (Utilities|Map|Find (Variables|Formula|Raw|GetActualEnemyHPMap) _enemytospawnclass)) _playerref self (Variables|/Script/Engine.ChildActorComponent|GetChildActor (Variables|/Game/Content/Characters/Player/MainCharacter_BP.MainCharacter_BP_C|GetFloor _playerref)) (Variables|Formula|Calc|GetCoeffDiff) (Variables|Formula|Calc|GetActualEnemyLevel)))
    (Math|Integer|IncrementInt (Variables|EnemySpawner|Other|GetEnemySpawned)
      (:%20%20
        (bind _returnvalue (Utilities|Array|Add (Variables|EnemySpawner|Other|GetEnemiesSpawned) _enemyspawned))
        (Variables|/Game/Content/Characters/Enemies/Enemy_MasterBP.Enemy_MasterBP_C|SetIndex _enemyspawned _returnvalue)))
    (else
      (Utilities|Time|ClearandInvalidateTimerbyHandle (Variables|EnemySpawner|Other|GetNormalWaveSpawnerHandle))
      (Variables|NormalWave|SetEnemiesToSpawn (+ (Variables|NormalWave|GetEnemiesToSpawn) (Variables|NormalWave|GetIncreaseEnemyToSpawnBy)))
      (Variables|EnemySpawner|Other|SetEnemySpawned 0)
      (Variables|Default|SetAllEnemySpawned true))))

(fn SpecialWave
  (if (> (Variables|SpecialWave|GetActualSpecialWaveTimer) 0)
    (if (not (== (Utilities|Array|Length (Variables|EnemySpawner|Other|GetEnemiesSpawned)) (Variables|SpecialWave|GetMaxEnemySpecialWave)))
      (CallFunction|SpawnSingleRandomEnemySpecialWave (.OutItem (Utilities|Array|Random (Variables|EnemySpawner|Other|GetEnemySpawners)))))
    (else
      (Variables|SpecialWave|SetSpecialWaveMultiplier (+ (Variables|SpecialWave|GetSpecialWaveMultiplier) 5))
      (Utilities|Time|ClearandInvalidateTimerbyHandle (Variables|SpecialWave|GetSpecialWaveSpawnerHandle))
      (Variables|EnemySpawner|Other|SetEnemySpawned 0))))

(fn CoefficenteDifficolta
  (bind _output_get (Variables|Formula|Calc|SetCoeffDiff (* (+ (Variables|Formula|Raw|GetPlayerFactor) (* (Variables|Formula|Raw|GetTimeInt) (Variables|Formula|Raw|GetTimeFactor))) (Math|Float|Power (Variables|Formula|Raw|GetStageFactor) (Math|Conversions|ToFloat(Integer) (Variables|Formula|Raw|GetCompletedStages))))))
  (return _output_get))

(fn EnemyLevel
  (params (CD :type Float%20%28double-precision%29))
  (Variables|Formula|Calc|SetActualEnemyLevel (/ (+ (- CD (Variables|Formula|Raw|GetPlayerFactor)) 1.0) (Variables|Formula|Raw|GetEnemyFactor)))
  (return))

(fn UpdateEnemyMapValue
  (bind _actualenemyhpmap (Variables|Formula|Raw|GetActualEnemyHPMap))
  (bind _actualenemyhpmap_2 (Variables|Formula|Raw|GetActualEnemyHPMap))
  (bind _value (Utilities|Map|Find _actualenemyhpmap "/Game/Content/Characters/Enemies/TankEnemy/TankEnemy_BP.TankEnemy_BP_C"))
  (bind _value_2 (Utilities|Map|Find _actualenemyhpmap_2 "/Game/Content/Characters/Enemies/GenericEnemy/GroundEnemy_BP.GroundEnemy_BP_C"))
  (Utilities|Map|Add _actualenemyhpmap_2 "/Game/Content/Characters/Enemies/GenericEnemy/GroundEnemy_BP.GroundEnemy_BP_C" (+ _value_2 (* _value_2 0.1)))
  (Utilities|Map|Add _actualenemyhpmap "/Game/Content/Characters/Enemies/TankEnemy/TankEnemy_BP.TankEnemy_BP_C" (+ _value (* _value 0.1)))
  (return))

(fn SpawnSingleRandomEnemySpecialWave
  (params (EnemySpawner :type Enemy%20Spawner%20BP%20Object%20Reference))
  (bind _enemytospawnclass (Variables|EnemySpawner|Other|GetEnemyToSpawnClass))
  (CallFunction|ChooseEnemytoSpawn)
  (bind _enemyspawned (Default|SpawnEnemy EnemySpawner _enemytospawnclass (.Value (Utilities|Map|Find (Variables|Formula|Raw|GetActualEnemyHPMap) _enemytospawnclass)) (Variables|Ref|GetPlayerRef) self (Variables|Ref|GetTimeMachineRef) (Variables|Formula|Calc|GetCoeffDiff) (Variables|Formula|Calc|GetActualEnemyLevel)))
  (Math|Integer|IncrementInt (Variables|EnemySpawner|Other|GetEnemySpawned)
    (:%20%20
      (bind _returnvalue (Utilities|Array|Add (Variables|EnemySpawner|Other|GetEnemiesSpawned) _enemyspawned))
      (Variables|/Game/Content/Characters/Enemies/Enemy_MasterBP.Enemy_MasterBP_C|SetIndex _enemyspawned _returnvalue))))