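; Rocket projectile for the rocket launcher that explodes on contact and deals area damage.
; On hit it activates the hit effect, spawns an impact actor, plays the explosion sound and destroys itself.
; A sphere trace at the hit point sends damage through TakeDamage_Interface, halved for the player referenced as PlayerRef, who is passed as damage causer.
; An unexploded rocket times out after a fixed delay, spawning the impact actor without dealing damage.
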(event OnComponentHit(Sphere1)
  (params (HitComponent :type Primitive%20Component%20Object%20Reference) (OtherActor :type Actor%20Object%20Reference) (OtherComp :type Primitive%20Component%20Object%20Reference) (NormalImpulse :type Vector :default "0, 0, 0") (Hit :type Hit%20Result%20Structure%20%28by%20ref%29))
  (bind _location (Collision|BreakHitResult Hit))
  (bind _hiteffects (Variables|Default|GetHiteffects))
  (bind _returnvalue (Math|Transform|MakeTransform _location "0, 0, 0" "3.000000,3.000000,3.000000"))
  (bind _location_2 (Math|Transform|BreakTransform _returnvalue))
  (Components|Activation|SetActive _hiteffects true false)
  (Transformation|SetWorldLocation _hiteffects _location false false)
  (Collision|SetCollisionEnabled (Variables|Default|GetSphere1) "NoCollision")
  (Game|SpawnActorfromClass (Variables|Default|GetImpactActor) _returnvalue "Undefined" 0 0)
  (Audio|PlaySoundatLocation "/Game/Content/Sounds/Weapons/Lanciarazzi/Esplosione_razzo.Esplosione_razzo" (Transformation|GetActorLocation) "0, 0, 0" 1.0 1.0 0.0 "/Game/Content/Sounds/SoundAttenuationSettings.SoundAttenuationSettings" 0 0 0)
  (bind _outhits (Collision|MultiSphereTraceByChannel _location_2 _location_2 3e+02 "TraceTypeQuery4" false 0 "None"))
  (for _array_element _outhits
    (if (Utilities|DoesObjectImplementInterface (.HitActor (Collision|BreakHitResult _array_element)) "/Game/Content/Characters/TakeDamage_Interface.TakeDamage_Interface_C")
      (if (== (.HitActor (Collision|BreakHitResult _array_element)) (Variables|Default|GetPlayerRef))
        (Class|TakeDamageInterface|TakeDamage(Message) (.HitActor (Collision|BreakHitResult _array_element)) (* (Variables|Default|GetDamage) 0.5) _array_element (Variables|Default|GetPlayerRef))
        (else
          (Class|TakeDamageInterface|TakeDamage(Message) (.HitActor (Collision|BreakHitResult _array_element)) (Variables|Default|GetDamage) _array_element (Variables|Default|GetPlayerRef))))))
  (Actor|DestroyActor))

(event EventBeginPlay
  (Class|NiagaraComponent|SetAsset (Variables|Default|GetHiteffects) (Variables|Default|GetHitEffect) true)
  (Utilities|FlowControl|Delay 1e+01)
  (Game|SpawnActorfromClass (Variables|Default|GetImpactActor) (Transformation|GetActorTransform) "Undefined" 0 0)
  (Actor|DestroyActor))

(fn ConstructionScript)