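; Rocket launcher weapon Blueprint that fires rockets from four muzzle points in rotation and knocks the player back.
; The construction script gathers the spawn components, and SelectSpawner cycles through their world locations.
; Each weapon action spawns a Rocket_BP along the camera rotation with player-scaled damage, plays a 2D sound and launches the character backward and upward.
; Shortly after BeginPlay it sets the UI max ammo display to zero.
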(event EventBeginPlay
  (|CallParentFunction)
  (Utilities|FlowControl|Delay 0.2)
  (Default|UpdateMaxAmmo (Variables|/Game/Content/Characters/Player/MainCharacter_BP.MainCharacter_BP_C|GetInGameUI (Variables|Default|GetPlayerRef))))

(event EventWeaponAction
  (bind _playerref (Variables|Default|GetPlayerRef))
  (bind _returnvalue (Transformation|GetActorForwardVector _playerref))
  (bind _returnvalue_2 (* _returnvalue -1e+03))
  (bind _transform (CallFunction|SelectSpawner))
  (Game|SpawnActorfromClass "/Game/Content/Gameplay/Weapons/Lanciarazzi/Rocket_BP.Rocket_BP_C" (Math|Transform|MakeTransform _transform (Camera|GetCameraRotation (Game|GetPlayerCameraManager 0)) "1.000000,1.000000,1.000000") "AlwaysSpawn" 0 (* (Variables|Default|GetDamage) (Variables|/Game/Content/Characters/Player/MainCharacter_BP.MainCharacter_BP_C|GetDamageMultiplier (Variables|Default|GetPlayerRef)) (Variables|/Game/Content/Characters/Player/MainCharacter_BP.MainCharacter_BP_C|GetPlayerLVLDMGMultiplier (Variables|Default|GetPlayerRef))) _playerref 0)
  (Audio|PlaySound2D "/Game/Content/Sounds/Weapons/Lanciarazzi/Lanciamissili.Lanciamissili" 1.0 1.0 0.0 0 0)
  (Character|LaunchCharacter _playerref (Math|Vector|MakeVector (.x _returnvalue_2) (.y _returnvalue_2) 2e+02) false false))

(fn ConstructionScript
  (|CallParentFunction)
  (Variables|Default|SetRocketSpawners (Utilities|Array|MakeArray (Variables|Default|GetRocketSpawn) (Variables|Default|GetRocketSpawn2) (Variables|Default|GetRocketSpawn3) (Variables|Default|GetRocketSpawn1))))

(fn SelectSpawner
  (LocalVariables|SetSelectedSpawnerLocation (Transformation|GetWorldLocation (Utilities|Array|Get(acopy) (Variables|Default|GetRocketSpawners) (Variables|Default|GetActualSpawnerIndex))))
  (bind _result (Math|Integer|IncrementInt (Variables|Default|GetActualSpawnerIndex))
    (:%20%20
      (if (not (> _result (Utilities|Array|LastIndex (Variables|Default|GetRocketSpawners))))
        _
        (else
          (Variables|Default|SetActualSpawnerIndex 0)))
      (return (LocalVariables|GetSelectedSpawnerLocation)))))