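; Master weapon Blueprint that serves as a base for weapons used by the player character.
; On BeginPlay it caches the player character, clears its reloading flag and binds use and release input to empty WeaponAction events, presumably for child overrides.
; A helper event spawns attached blood Niagara effects.
; GetImpactDecal and GetImpactFX switch on surface type but are unfinished, with no cases wired to their returns.
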(event Custom|PlayNiagaraFX
  (params (AttachTo :type Scene%20Component%20Object%20Reference) (BoneName :type Name) (Location :type Vector) (Rotation :type Vector))
  (Niagara|SpawnSystemAttached "/Game/Content/VFX/BloodSystem/NS_Blood.NS_Blood" AttachTo BoneName Location (Math|Conversions|RotationFromXVector Rotation) "KeepRelativeOffset" true))

(event Custom|WeaponAction
  ;[1 1 1] Begin play + default behaviour setup
)

(event Custom|WeaponActionReleased
  ;[1 1 1] Begin play + default behaviour setup
)

(event EventBeginPlay
  ;[1 1 1] Begin play + default behaviour setup
  (bind _asmain_character_bp (Utilities|Casting|CastToMainCharacter_BP (Game|GetPlayerCharacter 0)))
  (bind _output_get (Variables|Default|SetPlayerRef _asmain_character_bp))
  (Variables|/Game/Content/Characters/Player/MainCharacter_BP.MainCharacter_BP_C|SetisReloadingWeapon _output_get false)
  (EventDispatchers|BindEventtoOnUseItem _output_get (delegate Custom|WeaponAction))
  (EventDispatchers|BindEventtoOnUseReleased (Variables|Default|GetPlayerRef) (delegate Custom|WeaponActionReleased)))

(fn ConstructionScript)

(fn GetImpactDecal
  (params (SurfaceType :type EPhysicalSurface%20Enum :default "SurfaceType_Default"))
  (switch Utilities|FlowControl|Switch|SwitchonEPhysicalSurface SurfaceType))

(fn GetImpactFX
  (params (SurfaceType :type EPhysicalSurface%20Enum :default "SurfaceType_Default"))
  (switch Utilities|FlowControl|Switch|SwitchonEPhysicalSurface SurfaceType))