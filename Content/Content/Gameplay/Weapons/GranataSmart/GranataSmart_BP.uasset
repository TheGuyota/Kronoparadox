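; Smart grenade that, shortly after being thrown, rises into the air, seeks an enemy and explodes near it.
; A delayed timer removes the projectile component and plays a height timeline, then a looping box trace looks for an Enemy-tagged actor.
; A fast timer lerps the grenade toward that target.
; On proximity it spawns an impact actor, applies player-scaled sphere-trace damage through TakeDamage_Interface and destroys itself.
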(event Custom|CheckForEnemyInRange
  (bind _returnvalue (Transformation|GetActorLocation))
  (bind (_outhit _returnvalue_2) (Collision|BoxTraceByChannel _returnvalue _returnvalue "200.000000,200.000000,150.000000" "0, 0, 0" "TraceTypeQuery3" false 0 "None" true "(R=1.000000,G=0.000000,B=0.000000,A=1.000000)" "(R=0.000000,G=1.000000,B=0.000000,A=1.000000)" 0.5))
  (if _returnvalue_2
    (if (Actor|ActorHasTag (.HitActor (Collision|BreakHitResult _outhit)) "Enemy")
      (Variables|Default|SetActorToReach (.HitActor (Collision|BreakHitResult _outhit)))
      (Utilities|Time|SetTimerbyEvent (delegate Custom|ReachTarget) 0.01 true)
      (Utilities|Time|ClearandInvalidateTimerbyHandle (Variables|Default|GetCheckForEnemyHandle)))))

(event Custom|ReachTarget
  (bind _returnvalue (Transformation|GetActorLocation))
  (Transformation|SetActorLocation (Math|Vector|Lerp(Vector) (Transformation|GetActorLocation) (Transformation|GetActorLocation (Variables|Default|GetActorToReach)) 0.05) false false)
  (if (< (Math|Vector|Distance(Vector) (Transformation|GetActorLocation) (Transformation|GetActorLocation (Variables|Default|GetActorToReach))) 1e+02)
    (Game|SpawnActorfromClass (Variables|Default|GetImpactActor) (Math|Transform|MakeTransform (Transformation|GetActorLocation) "0, 0, 0" "1.000000,1.000000,1.000000") "AlwaysSpawn" 0 0)
    (bind _outhits (Collision|MultiSphereTraceByChannel _returnvalue _returnvalue 2e+02 "TraceTypeQuery4" false 0 "None" true "(R=1.000000,G=0.000000,B=0.000000,A=1.000000)" "(R=0.000000,G=1.000000,B=0.000000,A=1.000000)" 2.0))
    (for _array_element _outhits
      (if (Utilities|DoesObjectImplementInterface (.HitActor (Collision|BreakHitResult _array_element)) "/Game/Content/Characters/TakeDamage_Interface.TakeDamage_Interface_C")
        (Development|PrintString (Utilities|GetDisplayName (.HitActor (Collision|BreakHitResult _array_element))))
        (Class|TakeDamageInterface|TakeDamage(Message) (.HitActor (Collision|BreakHitResult _array_element)) (* (Variables|Default|GetGrenadeDamage) (Variables|/Game/Content/Characters/Player/MainCharacter_BP.MainCharacter_BP_C|GetDamageMultiplier (Variables|Default|GetPlayerRef)) (Variables|/Game/Content/Characters/Player/MainCharacter_BP.MainCharacter_BP_C|GetPlayerLVLDMGMultiplier (Variables|Default|GetPlayerRef))) _array_element (Variables|Default|GetPlayerRef))))
    (Actor|DestroyActor)))

(event Custom|Initialize
  (bind _returnvalue (Transformation|GetActorLocation))
  (Components|DestroyComponent (Variables|Default|GetProjectile))
  (Variables|Default|SetInitialZ (.z (Transformation|GetActorLocation)))
  (bind _zvalue (Timeline|GetUpInAir PlayFromStart)
    (:Update
      (Transformation|SetActorLocation (Math|Vector|MakeVector (.x _returnvalue) (.y _returnvalue) (+ (Variables|Default|GetInitialZ) _zvalue)) false false))
    (:Finished
      (bind _returnvalue_2 (Utilities|Time|SetTimerbyEvent (delegate Custom|CheckForEnemyInRange) 1.0 true))
      (Variables|Default|SetCheckForEnemyHandle _returnvalue_2))))

(event EventBeginPlay
  (Utilities|Time|SetTimerbyEvent (delegate Custom|Initialize) 2.0))

(fn ConstructionScript
  (|CallParentFunction))