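; Roccia_BP is a rock weapon actor that damages enemies on impact, apparently acting as a grenade-style projectile.
; BeginPlay assigns the Niagara hit effect, which activates when Sphere1 registers a hit.
; Actors tagged Enemy that implement TakeDamage_Interface receive grenade damage scaled by the player's damage and level multipliers.
; The actor destroys itself on any hit, immediately after activating the effect.
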(event OnComponentHit(Sphere1)
  (params (HitComponent :type Primitive%20Component%20Object%20Reference) (OtherActor :type Actor%20Object%20Reference) (OtherComp :type Primitive%20Component%20Object%20Reference) (NormalImpulse :type Vector :default "0, 0, 0") (Hit :type Hit%20Result%20Structure%20%28by%20ref%29))
  (bind _hitactor (Collision|BreakHitResult Hit))
  (Components|Activation|SetActive (Variables|Default|GetHiteffects) true false)
  (if (and (Utilities|DoesObjectImplementInterface _hitactor "/Game/Content/Characters/TakeDamage_Interface.TakeDamage_Interface_C") (Actor|ActorHasTag _hitactor "Enemy"))
    (Class|TakeDamageInterface|TakeDamage(Message) _hitactor (* (Variables|Default|GetGrenadeDamage) (Variables|/Game/Content/Characters/Player/MainCharacter_BP.MainCharacter_BP_C|GetDamageMultiplier (Variables|Default|GetPlayerRef)) (Variables|/Game/Content/Characters/Player/MainCharacter_BP.MainCharacter_BP_C|GetPlayerLVLDMGMultiplier (Variables|Default|GetPlayerRef))) Hit (Variables|Default|GetPlayerRef))
    (Actor|DestroyActor)
    (else
      (Actor|DestroyActor))))

(event EventBeginPlay
  (Class|NiagaraComponent|SetAsset (Variables|Default|GetHiteffects) (Variables|Default|GetHitEffect) true))

(fn ConstructionScript
  (|CallParentFunction))