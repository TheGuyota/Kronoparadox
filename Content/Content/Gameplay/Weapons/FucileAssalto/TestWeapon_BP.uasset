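; Automatic assault rifle Blueprint that fires while the weapon action is held, tracking ammo and the player's firing and reloading states.
; A looping timer repeats each shot at the fire rate, toggling muzzle FX, playing sound and spawning a projectile at the muzzle.
; A camera line trace separately applies damage through TakeDamage_Interface with a hit-marker sound.
; Reload events bound on the player set the reloading state and refill ammo.
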(event Custom|AutomaticFire
  (bind _muzzle (Variables|Default|GetMuzzle))
  (bind _playerref (Variables|Default|GetPlayerRef))
  (bind _firstpersoncamera (Variables|/Game/Content/Characters/Player/MainCharacter_BP.MainCharacter_BP_C|GetFirstPersonCamera _playerref))
  (bind _returnvalue (Transformation|GetWorldLocation _firstpersoncamera))
  (if (> (Variables|Default|GetActualAmmo) 0)
    (CallFunction|MuzzlefybcStop)
    (bind (_outhit _returnvalue_2) (Collision|LineTraceByChannel _returnvalue (+ _returnvalue (* (Math|Vector|GetForwardVector (Transformation|GetWorldRotation _firstpersoncamera)) 1e+04)) "TraceTypeQuery3" false 0 "None"))
    (CallFunction|MuzzlefybcStart)
    (Game|SpawnActorfromClass "/Game/Content/Gameplay/Weapons/FucileAssalto/ProiettileAssalto_BP.ProiettileAssalto_BP_C" (Math|Transform|MakeTransform (Transformation|GetWorldLocation _muzzle) (Transformation|GetWorldRotation _muzzle) "1.000000,1.000000,1.000000") "Undefined" 0 0)
    (Math|Integer|DecrementInt (Variables|Default|GetActualAmmo)
      (:%20%20
        (if _returnvalue_2
          (if (Utilities|DoesObjectImplementInterface (.HitActor (Collision|BreakHitResult _outhit)) "/Game/Content/Characters/TakeDamage_Interface.TakeDamage_Interface_C")
            (Audio|PlaySoundatLocation "/Game/Content/Sounds/Effects/HitMarker_Cue.HitMarker_Cue" (.Location (Collision|BreakHitResult _outhit)) "0, 0, 0" 1.0 1.0 0.0 0 0 0 0)
            (Class|TakeDamageInterface|TakeDamage(Message) (.HitActor (Collision|BreakHitResult _outhit)) (Variables|Default|GetDamage) _outhit (Variables|Default|GetPlayerRef))))))
    (else
      (Variables|/Game/Content/Characters/Player/MainCharacter_BP.MainCharacter_BP_C|SetisFiring (Variables|Default|GetPlayerRef) false)
      (Development|PrintString "No Ammo")
      (CallFunction|MuzzlefybcStop))))

(event Custom|ReloadWeapon
  (Variables|/Game/Content/Characters/Player/MainCharacter_BP.MainCharacter_BP_C|SetisReloadingWeapon (Variables|Default|GetPlayerRef) true))

(event Custom|ReloadEnd
  (Variables|Default|SetActualAmmo (Variables|Default|GetTotalAmmo))
  (Variables|/Game/Content/Characters/Player/MainCharacter_BP.MainCharacter_BP_C|SetisReloadingWeapon (Variables|Default|GetPlayerRef) false))

(event EventBeginPlay
  (|CallParentFunction)
  (EventDispatchers|BindEventtoReloadWeapon (Variables|Default|GetPlayerRef) (EventDispatchers|CreateEvent :!event Custom|ReloadWeapon))
  (EventDispatchers|BindEventtoWeaponReloaded (Variables|Default|GetPlayerRef) (EventDispatchers|CreateEvent :!event Custom|ReloadEnd)))

(event EventWeaponAction
  (if (> (Variables|Default|GetActualAmmo) 0)
    ;[1 1 1] FirstShot
    (CallFunction|AutomaticFire)
    (bind _returnvalue (Utilities|Time|SetTimerbyEvent (delegate Custom|AutomaticFire) (Variables|Default|GetFireRate) true))
    (Variables|/Game/Content/Characters/Player/MainCharacter_BP.MainCharacter_BP_C|SetisFiring (Variables|Default|GetPlayerRef) true)
    (Variables|Default|SetAutomaticFireHandle _returnvalue)
    (else
      (Development|PrintString "No Ammo"))))

(event EventWeaponActionReleased
  (Utilities|Time|ClearandInvalidateTimerbyHandle (Variables|Default|GetAutomaticFireHandle))
  (Variables|/Game/Content/Characters/Player/MainCharacter_BP.MainCharacter_BP_C|SetisFiring (Variables|Default|GetPlayerRef) false)
  (CallFunction|MuzzlefybcStop))

(fn ConstructionScript
  (|CallParentFunction))

(fn MuzzlefybcStart
  (bind _muzzle (Variables|Default|GetMuzzle))
  (Class|NiagaraComponent|SetAsset _muzzle (Variables|Default|GetMuzzleFX) true)
  (Components|Activation|SetActive _muzzle true false)
  (Audio|PlaySoundatLocation "/Game/Content/Sounds/Effects/FucileSparo_Cue.FucileSparo_Cue" (Transformation|GetWorldLocation (Variables|Default|GetMuzzle)) "0, 0, 0" 1.0 1.0 0.0 0 0 0 0))

(fn MuzzlefybcStop
  (bind _muzzle (Variables|Default|GetMuzzle))
  (Class|NiagaraComponent|SetAsset _muzzle 0 true)
  (Components|Activation|SetActive _muzzle false false))