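; Assault rifle weapon Blueprint that fires automatically while the weapon action is held, using a looping fire-rate timer.
; Each shot line-traces from the player camera for multiplier-scaled damage through TakeDamage_Interface, and also spawns a projectile from the muzzle toward the aim point.
; Muzzle effects, sounds and ammo UI updates accompany firing.
; Events bound to the player handle reloading, which refills the ammo to its total.
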(event Custom|AutomaticFire
  (bind _muzzle (Variables|Default|GetMuzzle))
  (bind _playerref (Variables|Default|GetPlayerRef))
  (bind _returnvalue (Transformation|GetWorldLocation _muzzle))
  (bind _firstpersoncamera (Variables|/Game/Content/Characters/Player/MainCharacter_BP.MainCharacter_BP_C|GetFirstPersonCamera _playerref))
  (bind _returnvalue_2 (Transformation|GetWorldLocation _firstpersoncamera))
  (bind _returnvalue_3 (Transformation|GetWorldRotation _firstpersoncamera))
  (bind _returnvalue_4 (Math|Vector|GetForwardVector _returnvalue_3))
  (bind _returnvalue_5 (* _returnvalue_4 8e+03))
  (bind _returnvalue_6 (+ _returnvalue_2 _returnvalue_5))
  (if (> (Variables|Default|GetActualAmmo) 0)
    (CallFunction|MuzzlefybcStop)
    (bind (_outhit _returnvalue_7) (Collision|LineTraceByChannel _returnvalue_2 _returnvalue_6 "TraceTypeQuery3" false 0 "None"))
    (CallFunction|MuzzlefybcStart)
    (Game|SpawnActorfromClass "/Game/Content/Gameplay/Weapons/FucileAssalto/ProiettileAssalto_BP.ProiettileAssalto_BP_C" (Math|Transform|MakeTransform _returnvalue (Math|Rotator|FindLookatRotation _returnvalue _returnvalue_6) "1.000000,1.000000,1.000000") "Undefined" 0 0)
    (Math|Integer|DecrementInt (Variables|Default|GetActualAmmo)
      (:%20%20
        (Default|UpdateCurrentAmmo (Variables|/Game/Content/Characters/Player/MainCharacter_BP.MainCharacter_BP_C|GetInGameUI (Variables|Default|GetPlayerRef)) (Variables|Default|GetActualAmmo))
        (if _returnvalue_7
          (if (Utilities|DoesObjectImplementInterface (.HitActor (Collision|BreakHitResult _outhit)) "/Game/Content/Characters/TakeDamage_Interface.TakeDamage_Interface_C")
            (Audio|PlaySoundatLocation "/Game/Content/Sounds/Effects/HitMarker_Cue.HitMarker_Cue" (.Location (Collision|BreakHitResult _outhit)) "0, 0, 0" 0.3 1.0 0.0 "/Game/Content/Sounds/SoundAttenuationSettings.SoundAttenuationSettings" 0 0 0)
            (Class|TakeDamageInterface|TakeDamage(Message) (.HitActor (Collision|BreakHitResult _outhit)) (* (Variables|Default|GetDamage) (Variables|/Game/Content/Characters/Player/MainCharacter_BP.MainCharacter_BP_C|GetDamageMultiplier (Variables|Default|GetPlayerRef)) (Variables|/Game/Content/Characters/Player/MainCharacter_BP.MainCharacter_BP_C|GetPlayerLVLDMGMultiplier (Variables|Default|GetPlayerRef))) _outhit (Variables|Default|GetPlayerRef))))))
    (else
      (Variables|/Game/Content/Characters/Player/MainCharacter_BP.MainCharacter_BP_C|SetisFiring (Variables|Default|GetPlayerRef) false)
      (Development|PrintString "No Ammo")
      (CallFunction|MuzzlefybcStop))))

(event Custom|ReloadWeapon
  (if (< (Variables|Default|GetActualAmmo) (Variables|Default|GetTotalAmmo))
    (Variables|/Game/Content/Characters/Player/MainCharacter_BP.MainCharacter_BP_C|SetisReloadingWeapon (Variables|Default|GetPlayerRef) true)
    (Audio|PlaySoundatLocation "/Game/Content/Sounds/Weapons/Fucile/Fucile_Ricarica.Fucile_Ricarica" (Transformation|GetActorLocation) "0, 0, 0" 1.0 1.0 0.1 0 0 0 0)))

(event Custom|ReloadEnd
  (Variables|Default|SetActualAmmo (Variables|Default|GetTotalAmmo))
  (Variables|/Game/Content/Characters/Player/MainCharacter_BP.MainCharacter_BP_C|SetisReloadingWeapon (Variables|Default|GetPlayerRef) false)
  (Default|UpdateCurrentAmmo (Variables|/Game/Content/Characters/Player/MainCharacter_BP.MainCharacter_BP_C|GetInGameUI (Variables|Default|GetPlayerRef)) (Variables|Default|GetActualAmmo)))

(event EventBeginPlay
  (bind _playerref (Variables|Default|GetPlayerRef))
  (bind _ingameui (Variables|/Game/Content/Characters/Player/MainCharacter_BP.MainCharacter_BP_C|GetInGameUI _playerref))
  (|CallParentFunction)
  (EventDispatchers|BindEventtoReloadWeapon (Variables|Default|GetPlayerRef) (EventDispatchers|CreateEvent :!event Custom|ReloadWeapon))
  (EventDispatchers|BindEventtoWeaponReloaded (Variables|Default|GetPlayerRef) (EventDispatchers|CreateEvent :!event Custom|ReloadEnd))
  (Utilities|FlowControl|Delay 0.2)
  (Default|UpdateMaxAmmo _ingameui (Variables|Default|GetTotalAmmo))
  (Default|UpdateCurrentAmmo _ingameui (Variables|Default|GetActualAmmo)))

(event EventWeaponAction
  (if (> (Variables|Default|GetActualAmmo) 0)
    ;[1 1 1] FirstShot
    (CallFunction|AutomaticFire)
    (bind _returnvalue (Utilities|Time|SetTimerbyEvent (delegate Custom|AutomaticFire) (Variables|Default|GetFireRate) true))
    (Variables|/Game/Content/Characters/Player/MainCharacter_BP.MainCharacter_BP_C|SetisFiring (Variables|Default|GetPlayerRef) true)
    (Variables|Default|SetAutomaticFireHandle _returnvalue)
    (else
      (Development|PrintString "No Ammo"))))

(event EventWeaponActionReleased
  (Utilities|Time|ClearandInvalidateTimerbyHandle (Variables|Default|GetAutomaticFireHandle))
  (Variables|/Game/Content/Characters/Player/MainCharacter_BP.MainCharacter_BP_C|SetisFiring (Variables|Default|GetPlayerRef) false)
  (CallFunction|MuzzlefybcStop))

(fn ConstructionScript
  (|CallParentFunction))

(fn MuzzlefybcStart
  (bind _muzzle (Variables|Default|GetMuzzle))
  (Class|NiagaraComponent|SetAsset _muzzle (Variables|Default|GetMuzzleFX) true)
  (Components|Activation|SetActive _muzzle true false)
  (Audio|PlaySoundatLocation "/Game/Content/Sounds/Effects/FucileSparo_Cue.FucileSparo_Cue" (Transformation|GetWorldLocation (Variables|Default|GetMuzzle)) "0, 0, 0" 0.2 1.0 0.0 0 0 0 0))

(fn MuzzlefybcStop
  (bind _muzzle (Variables|Default|GetMuzzle))
  (Class|NiagaraComponent|SetAsset _muzzle 0 true)
  (Components|Activation|SetActive _muzzle false false))