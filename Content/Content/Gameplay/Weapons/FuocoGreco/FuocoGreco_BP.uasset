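; FuocoGreco_BP is a thrown Greek fire grenade that damages enemies and leaves a fire pit where it breaks.
; On hit, it damages Enemy-tagged actors, scaling grenade damage by the player's damage and level multipliers.
; Every impact spawns a FirePit_BP at the FireLocation component, plays the breaking sound and destroys the grenade.
; Tick holds the SpringArm at a fixed world rotation, independent of the grenade's rotation.
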(event Collision|EventHit
  (params (MyComp :type Primitive%20Component%20Object%20Reference) (Other :type Actor%20Object%20Reference) (OtherComp :type Primitive%20Component%20Object%20Reference) (bSelfMoved :type Boolean) (HitLocation :type Vector :default "0, 0, 0") (HitNormal :type Vector :default "0, 0, 0") (NormalImpulse :type Vector :default "0, 0, 0") (Hit :type Hit%20Result%20Structure%20%28by%20ref%29))
  (bind _hitactor (Collision|BreakHitResult Hit))
  (bind _firelocation (Variables|Default|GetFireLocation))
  (bind _returnvalue (Transformation|GetWorldLocation _firelocation))
  (if (Actor|ActorHasTag _hitactor "Enemy")
    (Class|TakeDamageInterface|TakeDamage(Message) _hitactor (* (Variables|Default|GetGrenadeDamage) (Variables|/Game/Content/Characters/Player/MainCharacter_BP.MainCharacter_BP_C|GetDamageMultiplier (Variables|Default|GetPlayerRef)) (Variables|/Game/Content/Characters/Player/MainCharacter_BP.MainCharacter_BP_C|GetPlayerLVLDMGMultiplier (Variables|Default|GetPlayerRef))) Hit (Variables|Default|GetPlayerRef)))
  (bind _returnvalue_2 (Game|SpawnActorfromClass "/Game/Content/Gameplay/Weapons/FuocoGreco/FirePit_BP.FirePit_BP_C" (Math|Transform|MakeTransform _returnvalue "0, 0, 0" "1.000000,1.000000,1.000000") "Undefined" 0 (Variables|Default|GetPlayerRef) 0))
  (Default|CreateFirePit _returnvalue_2 _returnvalue)
  (Audio|PlaySoundatLocation "/Game/Content/Sounds/Weapons/Fuoco_Greco/Fuoco_greco_si_rompe.Fuoco_greco_si_rompe" (Transformation|GetActorLocation) "0, 0, 0" 0.35 1.0 0.0 "/Game/Content/Sounds/SoundAttenuationSettings.SoundAttenuationSettings" 0 0 0)
  (Actor|DestroyActor))

(event EventTick
  (params (DeltaSeconds :type Float%20%28single-precision%29))
  (Transformation|SetWorldRotation (Variables|Default|GetSpringArm) "90.000000, 0, 0" false false))

(fn ConstructionScript
  (|CallParentFunction))