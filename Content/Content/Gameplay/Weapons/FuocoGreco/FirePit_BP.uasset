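; FirePit_BP is a Greek fire (FuocoGreco) weapon hazard that leaves a temporary damaging fire at a given location.
; CreateFirePit spawns a randomly scaled Niagara fire, starts a looping damage timer and schedules StopFire after a random duration.
; Each tick sphere-traces at the fire, sending player-scaled damage through TakeDamage_Interface and skipping consecutive repeat hits on one actor.
; StopFire removes the effect and destroys the actor.
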(event Custom|StartFireDamage
  (bind _activefireeffects (Variables|Default|GetActiveFireEffects))
  (bind _returnvalue (Transformation|GetWorldLocation _activefireeffects))
  (Variables|Default|SetLastHitActor 0)
  (bind _outhits (Collision|MultiSphereTraceByChannel _returnvalue _returnvalue 2.2e+02 "TraceTypeQuery4" false 0 "None" true "(R=1.000000,G=0.000000,B=0.000000,A=1.000000)" "(R=0.000000,G=1.000000,B=0.000000,A=1.000000)" 0.5))
  (for _array_element _outhits
    (if (Utilities|DoesObjectImplementInterface (.HitActor (Collision|BreakHitResult _array_element)) "/Game/Content/Characters/TakeDamage_Interface.TakeDamage_Interface_C")
      (if (not (== (.HitActor (Collision|BreakHitResult _array_element)) (Variables|Default|GetLastHitActor)))
        (bind _output_get (Variables|Default|SetLastHitActor (.HitActor (Collision|BreakHitResult _array_element))))
        (Class|TakeDamageInterface|TakeDamage(Message) _output_get (* (Variables|Default|GetFirePitDamage) (Variables|/Game/Content/Characters/Player/MainCharacter_BP.MainCharacter_BP_C|GetDamageMultiplier (Variables|Default|GetPlayerRef)) (Variables|/Game/Content/Characters/Player/MainCharacter_BP.MainCharacter_BP_C|GetPlayerLVLDMGMultiplier (Variables|Default|GetPlayerRef))) _array_element (Variables|Default|GetPlayerRef))))))

(event Custom|CreateFirePit
  (params (FireLocation :type Vector))
  (bind _returnvalue (Niagara|SpawnSystematLocation "/Game/SFX/Particles/Fire_NS.Fire_NS" FireLocation "0, 0, 0" (Math|Vector|MakeVector (Math|Random|RandomFloatinRange 15.0 3e+01) (Math|Random|RandomFloatinRange 15.0 3e+01) 1.0)))
  (Variables|Default|SetActiveFireEffects _returnvalue)
  (bind _returnvalue_2 (Utilities|Time|SetTimerbyEvent (delegate Custom|StartFireDamage) 1.0 true))
  (Variables|Default|SetFireDamageHandle _returnvalue_2)
  (Utilities|Time|SetTimerbyEvent (delegate Custom|StopFire) (Math|Random|RandomFloatinRange (Variables|Default|GetFireDurationMin) (Variables|Default|GetFireDurationMax))))

(event Custom|StopFire
  (Development|PrintString "FireEnded")
  (Components|DestroyComponent (Variables|Default|GetActiveFireEffects))
  (Actor|DestroyActor))

(fn ConstructionScript)