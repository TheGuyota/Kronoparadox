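; Crossbow bolt projectile that damages what it hits and sticks in place.
; On box overlap, targets implementing TakeDamage_Interface take damage credited to the player, and the bolt attaches to them with an impact sound.
; Other hits play a different sound.
; Either way it removes its movement and collision and expires after a short lifespan, while a looping timer is meant to destroy it earlier if the attached enemy disappears.
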(event OnComponentBeginOverlap(Box)
  (params (OverlappedComponent :type Primitive%20Component%20Object%20Reference) (OtherActor :type Actor%20Object%20Reference) (OtherComp :type Primitive%20Component%20Object%20Reference) (OtherBodyIndex :type Integer) (bFromSweep :type Boolean) (SweepResult :type Hit%20Result%20Structure%20%28by%20ref%29))
  ;[1 1 1] Attach arrow to enemy and destroy with him or wait N seconds to destroy
  (if (Utilities|DoesObjectImplementInterface OtherActor "/Game/Content/Characters/TakeDamage_Interface.TakeDamage_Interface_C")
    (Transformation|AttachActorToActor self OtherActor "None" "KeepWorld" "KeepWorld" "KeepWorld" true)
    (Utilities|Time|SetTimerbyEvent (EventDispatchers|CreateEvent :!event Custom|DestroyWithEnemy) 0.1 true)
    (Audio|PlaySoundatLocation "/Game/Content/Sounds/Weapons/Balestra/Dardo_conficcato_1.Dardo_conficcato_1" (Transformation|GetActorLocation) "0, 0, 0" 0.1 1.0 0.0 0 0 0 0)
    (Class|TakeDamageInterface|TakeDamage(Message) :self OtherActor :DamageReceived (Variables|Default|GetDMG) :DamageCauser (Variables|Default|GetPlayerRef))
    (Variables|Default|GetProjectileMovement
      (:then
        _)
      (:else))
    (else
      (Audio|PlaySoundatLocation "/Game/Content/Sounds/Weapons/Balestra/Dardo_conficcato_2.Dardo_conficcato_2" (Transformation|GetActorLocation) "0, 0, 0" 0.1 1.0 0.0 0 0 0 0)))
  (Components|DestroyComponent (Variables|Default|GetProjectileMovement))
  (Components|DestroyComponent (Variables|Default|GetBox))
  (Actor|SetLifeSpan 3.0))

(event Custom|DestroyWithEnemy
  ;[1 1 1] Attach arrow to enemy and destroy with him or wait N seconds to destroy
  (Utilities|IsValid (stale OnComponentBeginOverlap(Box) OtherActor)
    (:Is%20Not%20Valid
      (Actor|DestroyActor))))

(fn ConstructionScript)