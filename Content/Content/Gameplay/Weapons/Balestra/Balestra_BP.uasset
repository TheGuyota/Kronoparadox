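; Crossbow (Balestra) weapon Blueprint that auto-fires volleys of three Dardo_BP darts in a yaw fan from spawner components, aimed by the player's camera.
; Pressing fire starts a looping timer behind a short anti-spam gate, and releasing clears it.
; A DoN node caps volleys per magazine, with damage scaled by player multipliers.
; Reload events bound to the player reset the counter and ammo, which feeds the in-game UI.
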(event Custom|Fire
  (bind _playerref (Variables|Default|GetPlayerRef))
  (bind _firstpersoncamera (Variables|/Game/Content/Characters/Player/MainCharacter_BP.MainCharacter_BP_C|GetFirstPersonCamera _playerref))
  (bind _returnvalue (Transformation|GetWorldRotation _firstpersoncamera))
  ;[1 1 1] Automatic fire + single fire event
  (Utilities|FlowControl|DoN 6
    (:Exit
      (if (Variables|Default|GetcanShoot)
        (Audio|PlaySoundatLocation "/Game/Content/Sounds/Weapons/Balestra/Balestra_scocco.Balestra_scocco" (Transformation|GetActorLocation) "0, 0, 0" 1.0 1.0 0.0 0 0 0 0)
        (for (_array_element _array_index) (Variables|Default|GetArrowSpawners)
          (Game|SpawnActorfromClass "/Game/Content/Gameplay/Weapons/Balestra/Dardo_BP.Dardo_BP_C" (Math|Transform|MakeTransform (Transformation|GetWorldLocation _array_element) (Math|Rotator|MakeRotator (.roll _returnvalue) (.pitch _returnvalue) (+ (.yaw _returnvalue) (Variables|Default|GetRotationZOffset))) "1.000000,1.000000,1.000000") "AlwaysSpawn" 0 (Variables|Default|GetPlayerRef) (* (Variables|Default|GetDamage) (Variables|/Game/Content/Characters/Player/MainCharacter_BP.MainCharacter_BP_C|GetDamageMultiplier (Variables|Default|GetPlayerRef)) (Variables|/Game/Content/Characters/Player/MainCharacter_BP.MainCharacter_BP_C|GetPlayerLVLDMGMultiplier (Variables|Default|GetPlayerRef))) 0)
          (switch int _array_index
            (:0
              (Variables|Default|SetRotationZOffset 3.5))
            (:1
              (Variables|Default|SetRotationZOffset -3.5))
            (:2
              (Variables|Default|SetRotationZOffset 0.0))))
        (bind _output_get (Variables|Default|SetCurrentAmmo (- (Variables|Default|GetCurrentAmmo) 3)))
        (Default|UpdateCurrentAmmo (Variables|/Game/Content/Characters/Player/MainCharacter_BP.MainCharacter_BP_C|GetInGameUI (Variables|Default|GetPlayerRef)) _output_get)
        (if (== (Variables|Default|GetCurrentAmmo) 0)
          (Variables|Default|SetcanShoot false))))))

(event Custom|ReloadEnd
  (bind _playerref (Variables|Default|GetPlayerRef))
  (bind _firstpersoncamera (Variables|/Game/Content/Characters/Player/MainCharacter_BP.MainCharacter_BP_C|GetFirstPersonCamera _playerref))
  (bind _returnvalue (Transformation|GetWorldRotation _firstpersoncamera))
  ;[1 1 1] Automatic fire + single fire event
  (Variables|Default|SetcanShoot true)
  (Variables|/Game/Content/Characters/Player/MainCharacter_BP.MainCharacter_BP_C|SetisReloadingWeapon (Variables|Default|GetPlayerRef) false)
  (Utilities|FlowControl|Sequence
    (:then_0
      (Utilities|FlowControl|DoN 6) ; enters at Reset
    )
    (:then_1
      (bind _output_get (Variables|Default|SetCurrentAmmo (Variables|Default|GetMaxAmmo)))
      (Default|UpdateCurrentAmmo (Variables|/Game/Content/Characters/Player/MainCharacter_BP.MainCharacter_BP_C|GetInGameUI (Variables|Default|GetPlayerRef)) _output_get))))

(event Custom|ReloadStart
  ;[1 1 1] Reload start
  (if (< (Variables|Default|GetCurrentAmmo) (Variables|Default|GetMaxAmmo))
    (Variables|/Game/Content/Characters/Player/MainCharacter_BP.MainCharacter_BP_C|SetisReloadingWeapon (Variables|Default|GetPlayerRef) true)
    (Audio|PlaySoundatLocation "/Game/Content/Sounds/Weapons/Balestra/Ricarica_balestra.Ricarica_balestra" (Transformation|GetActorLocation) "0, 0, 0" 1.0 1.0 0.1 0 0 0 0)))

(event Custom|ManualDelay
  ;[1 1 1] Automatic fire + single fire event
  (Variables|Default|SetFireRatePassed true))

(event EventBeginPlay
  (bind _playerref (Variables|Default|GetPlayerRef))
  (bind _ingameui (Variables|/Game/Content/Characters/Player/MainCharacter_BP.MainCharacter_BP_C|GetInGameUI _playerref))
  ;[1 1 1] Begin play + bind
  (|CallParentFunction)
  (Utilities|FlowControl|Delay 0.2)
  (Default|UpdateMaxAmmo _ingameui 18)
  (Default|UpdateCurrentAmmo _ingameui 18)
  (EventDispatchers|BindEventtoWeaponReloaded (Variables|Default|GetPlayerRef) (EventDispatchers|CreateEvent :!event Custom|ReloadEnd))
  (EventDispatchers|BindEventtoReloadWeapon (Variables|Default|GetPlayerRef) (EventDispatchers|CreateEvent :!event Custom|ReloadStart)))

(event EventWeaponActionReleased
  ;[1 1 1] Stop automatic fire
  (Utilities|Time|ClearandInvalidateTimerbyHandle (Variables|Default|GetFireHandle)))

(event EventWeaponAction
  ;[1 1 1] Automatic fire + single fire event
  (if (Variables|Default|GetFireRatePassed)
    (Utilities|FlowControl|Sequence
      (:then_0
        (Variables|Default|SetFireRatePassed false)
        (Utilities|Time|SetTimerbyEvent (delegate Custom|ManualDelay) 0.5))
      (:then_1
        (bind _returnvalue (Utilities|Time|SetTimerbyEvent (delegate Custom|Fire) (Variables|Default|GetFireRate) true -0.5))
        (Variables|Default|SetFireHandle _returnvalue)))))

(fn ConstructionScript
  (|CallParentFunction)
  (Variables|Default|SetArrowSpawners (Utilities|Array|MakeArray (Variables|Default|GetArrowSpawner1) (Variables|Default|GetArrowSpawner2) (Variables|Default|GetArrowSpawner))))