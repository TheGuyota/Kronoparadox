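; Grenade weapon actor that explodes on a timer and deals area damage.
; BeginPlay starts the fuse timer, and collision hits briefly move and activate a hit effect at the contact point.
; The explosion spawns an impact actor, plays a sound and sphere-traces around itself, then destroys the grenade.
; Traced actors implementing TakeDamage_Interface receive grenade damage scaled by the player's damage and level multipliers.
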(event OnComponentHit(Sphere1)
  (params (HitComponent :type Primitive%20Component%20Object%20Reference) (OtherActor :type Actor%20Object%20Reference) (OtherComp :type Primitive%20Component%20Object%20Reference) (NormalImpulse :type Vector :default "0, 0, 0") (Hit :type Hit%20Result%20Structure%20%28by%20ref%29))
  (bind _hiteffects (Variables|Default|GetHiteffects))
  ;[1 1 1] HitEffect
  (Components|Activation|SetActive _hiteffects true false)
  (Transformation|SetWorldLocation _hiteffects (.Location (Collision|BreakHitResult Hit)) false false)
  (Utilities|FlowControl|Delay 0.2)
  (Components|Activation|SetActive (Variables|Default|GetHiteffects) false false))

(event Custom|Explosion
  (bind _returnvalue (Transformation|GetActorLocation))
  ;[1 1 1] Explosion
  (Game|SpawnActorfromClass (Variables|Default|GetImpactActor) (Math|Transform|MakeTransform _returnvalue "0, 0, 0" "1.000000,1.000000,1.000000") "AlwaysSpawn" 0 0)
  (Audio|PlaySoundatLocation "/Game/Content/Sounds/Weapons/Granata/Esplosione_Granata_.Esplosione_Granata_" (Transformation|GetActorLocation) "0, 0, 0" 1.0 1.0 0.0 "/Game/Content/Sounds/SoundAttenuationSettings.SoundAttenuationSettings" 0 0 0)
  (bind _outhits (Collision|MultiSphereTraceByChannel _returnvalue _returnvalue 2e+02 "TraceTypeQuery4" false 0 "None" true "(R=1.000000,G=0.000000,B=0.000000,A=1.000000)" "(R=0.000000,G=1.000000,B=0.000000,A=1.000000)" 3.0))
  (for _array_element _outhits
    (if (Utilities|DoesObjectImplementInterface (.HitActor (Collision|BreakHitResult _array_element)) "/Game/Content/Characters/TakeDamage_Interface.TakeDamage_Interface_C")
      (Class|TakeDamageInterface|TakeDamage(Message) (.HitActor (Collision|BreakHitResult _array_element)) (* (Variables|Default|GetGrenadeDamage) (Variables|/Game/Content/Characters/Player/MainCharacter_BP.MainCharacter_BP_C|GetDamageMultiplier (Variables|Default|GetPlayerRef)) (Variables|/Game/Content/Characters/Player/MainCharacter_BP.MainCharacter_BP_C|GetPlayerLVLDMGMultiplier (Variables|Default|GetPlayerRef))) _array_element (Variables|Default|GetPlayerRef))))
  (Actor|DestroyActor))

(event EventBeginPlay
  ;[1 1 1] BeginPlay
  (|CallParentFunction)
  (Class|NiagaraComponent|SetAsset (Variables|Default|GetHiteffects) (Variables|Default|GetHitEffect) true)
  (Utilities|Time|SetTimerbyEvent (EventDispatchers|CreateEvent :!event Custom|Explosion) (Variables|Default|GetGrenadeTimer)))

(fn ConstructionScript
  (|CallParentFunction))